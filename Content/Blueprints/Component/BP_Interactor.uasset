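; Actor component that lets its owner aim at and start interactions with actors carrying a BP_Interactable component.
; Tick runs only for the local net owner, sphere tracing from the owner's eyes to track the current hit.
; Hit or interactability changes send aim started, updated or ended notifications and update AimedInteractable.
; StartInteraction calls a server event, which re-traces and rechecks CanInteract rather than using the passed interactable.
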(event Custom|SV_StartInteraction
  (params (Interactable :type BP%20Interactable%20Object%20Reference%20%28by%20ref%29))
  (bind _hitresult (CallFunction|QueryAimTrace))
  (Utilities|IsValid (CallFunction|GetInteractablefromHitResult _hitresult)
    (:Is%20Valid
      (if (Default|CanInteract (CallFunction|GetInteractablefromHitResult _hitresult) self)
        (Default|NotifyInteractionStarted (CallFunction|GetInteractablefromHitResult _hitresult) self)))))

(event EventBeginPlay
  (bind _returnvalue (Class|BPIActor|HasLocalNetOwnerBP(Message) (Components|GetOwner)))
  (Components|Tick|SetComponentTickEnabled _returnvalue))

(event EventTick
  (params (DeltaSeconds :type Float%20%28single-precision%29))
  (CallFunction|UpdateCurrentHit)
  (CallFunction|TryNotifyAimUpdates)
  (Variables|Default|SetbWasPreviousHitInteractable (CallFunction|IsInteractableHit (Variables|Default|GetCurrentHit))))

(fn StartInteraction
  (bind _aimedinteractable (Variables|Default|GetAimedInteractable)
    (:then
      (if (Default|CanInteract _aimedinteractable self)
        (CallFunction|SVStartInteraction (Variables|Default|GetAimedInteractable))))
    (:else)))

(fn QueryAimTrace
  (bind (_outlocation _outrotation) (Class|BPIActor|GetActorEyesViewPointBP(Message) (Components|GetOwner)))
  (bind _outhit (Collision|SphereTraceByChannel _outlocation (+ _outlocation (* (Math|Vector|GetForwardVector _outrotation) (Variables|Config|GetAimDistance))) 1.0 "TraceTypeQuery1" false 0 "ForOneFrame"))
  (return _outhit))

(fn UpdateCurrentHit
  (Variables|Default|SetPreviousHit (Variables|Default|GetCurrentHit))
  (bind _hitresult (CallFunction|QueryAimTrace))
  (Variables|Default|SetCurrentHit _hitresult))

(fn TryNotifyAimUpdates
  (if (CallFunction|IsHitUpdated)
    (LocalVariables|SetCurrent (CallFunction|GetInteractablefromHitResult (Variables|Default|GetCurrentHit)))
    (LocalVariables|SetPrevious (CallFunction|GetInteractablefromHitResult (Variables|Default|GetPreviousHit)))
    (bind _previous (LocalVariables|GetPrevious)
      (:then
        (if (== _previous (LocalVariables|GetCurrent))
          (Default|NotifyAimUpdated (LocalVariables|GetPrevious))
          (else
            (Default|NotifyAimEnded (LocalVariables|GetPrevious))
            (bind _output_get (Variables|Default|SetAimedInteractable (LocalVariables|GetCurrent) :!label _label))
            (Utilities|IsValid _output_get
              (:Is%20Valid
                (Default|NotifyAimStarted _output_get))))))
      (:else
        (goto _label)))))

(fn IsHitUpdated
  (bind _previoushit (Variables|Default|GetPreviousHit))
  (bind _currenthit (Variables|Default|GetCurrentHit))
  (bind (_bblockinghit _binitialoverlap _time _distance _location _impactpoint _normal _impactnormal _physmat _hitactor _hitcomponent _hitbonename) (Collision|BreakHitResult _currenthit))
  (bind (_bblockinghit_2 _binitialoverlap_2 _time_2 _distance_2 _location_2 _impactpoint_2 _normal_2 _impactnormal_2 _physmat_2 _hitactor_2 _hitcomponent_2 _hitbonename_2) (Collision|BreakHitResult _previoushit))
  (return (Math|Boolean|ORBoolean (!= _bblockinghit_2 _bblockinghit) (!= _hitactor_2 _hitactor) (!= _hitcomponent_2 _hitcomponent) (!= _hitbonename_2 _hitbonename) (!= (Variables|Default|GetbWasPreviousHitInteractable) (CallFunction|IsInteractableHit (Variables|Default|GetCurrentHit))))))

(fn IsInteractableHit
  (params (HitResult :type Hit%20Result%20Structure%20%28by%20ref%29))
  (bind _hitactor (Collision|BreakHitResult HitResult))
  (bind _returnvalue (Actor|GetComponentbyClass _hitactor "/Game/Blueprints/Component/BP_Interactable.BP_Interactable_C"))
  (Utilities|IsValid _hitactor
    (:Is%20Valid
      (Utilities|IsValid _returnvalue
        (:Is%20Valid
          (return (Default|CanInteract _returnvalue self)))))))

(fn GetInteractablefromHitResult
  (params (HitResult :type Hit%20Result%20Structure%20%28by%20ref%29))
  (bind _hitactor (Collision|BreakHitResult HitResult))
  (Utilities|IsValid _hitactor
    (:Is%20Valid
      (return (Actor|GetComponentbyClass _hitactor "/Game/Blueprints/Component/BP_Interactable.BP_Interactable_C")))))