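; BP_ControlPanel is an interactable three-button panel (Left, Right, Enter) for cycling through a set of options and confirming.
; On BeginPlay the authority registers each button as a labeled aim component with BPInteractable.
; Interactions fire per-button events, with Left and Right stepping a wrapping SelectedIndex whose OnRep announces selection updates.
; The click sound goes through MC_PlaySoundLocally, playing only for the interactor's local net owner.
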(event OnInteractionStarted(BP_Interactable)
  (params (Interactor :type BP%20Interactor%20Object%20Reference) (Component :type Primitive%20Component%20Object%20Reference))
  (Utilities|FlowControl|Sequence
    (:then_0
      (if (== Component (Variables|Default|GetButton_Left))
        (Default|CallOnLeftButtonPressed)
        (CallFunction|DecrementIndex)
        (CallFunction|MCPlaySoundLocally Interactor "/Engine/VREditor/Sounds/UI/Click_on_Button_Cue.Click_on_Button_Cue" :!label _label)))
    (:then_1
      (if (== Component (Variables|Default|GetButton_Right))
        (Default|CallOnRightButtonPressed)
        (CallFunction|IncrementIndex)
        (goto _label)))
    (:then_2
      (if (== Component (Variables|Default|GetButton_Enter))
        (Default|CallOnEnterButtonPressed)
        (goto _label)))))

(event Custom|MC_PlaySoundLocally
  (params (TargetPlayerContext :type BP%20Interactor%20Object%20Reference) (Sound :type Sound%20Base%20Object%20Reference))
  (Utilities|IsValid TargetPlayerContext
    (:Is%20Valid
      (bind _returnvalue (Class|BPIActor|HasLocalNetOwnerBP(Message) (Components|GetOwner TargetPlayerContext)))
      (if _returnvalue
        (Audio|PlaySoundatLocation Sound (Transformation|GetActorLocation) "0, 0, 0" 1.0 1.0 0.0 0 0 0 0)))))

(event EventBeginPlay
  (Networking|SwitchHasAuthority
    (:Authority
      (Default|SVRegisterAimComponent (Variables|Default|GetBP_Interactable) (Variables|Default|GetButton_Left))
      (Default|SVRegisterAimComponent (Variables|Default|GetBP_Interactable) (Variables|Default|GetButton_Right))
      (Default|SVRegisterAimComponent (Variables|Default|GetBP_Interactable) (Variables|Default|GetButton_Enter))
      (Default|SVRegisterAimLabel (Variables|Default|GetBP_Interactable) (Variables|Default|GetButton_Left) "ButtonLabel_Left")
      (Default|SVRegisterAimLabel (Variables|Default|GetBP_Interactable) (Variables|Default|GetButton_Right) "ButtonLabel_Right")
      (Default|SVRegisterAimLabel (Variables|Default|GetBP_Interactable) (Variables|Default|GetButton_Enter) "ButtonLabel_Enter"))))

(fn ConstructionScript)

(fn GetSelectedIndex
  (return (Variables|Default|GetSelectedIndex)))

(fn SetOptionCount
  (params (OptionCount :type Integer))
  (bind _output_get (Variables|Default|SetOptionCount OptionCount))
  (CallFunction|SetIndex (Math|Integer|SelectInt 0 (Variables|Default|GetINVALID_INDEX) (> _output_get 0))))

(fn OnRepSelectedIndex
  (Default|CallOnSelectionUpdated (Variables|Default|GetSelectedIndex)))

(fn IncrementIndex
  (CallFunction|SetIndex (+ (Variables|Default|GetSelectedIndex) 1)))

(fn DecrementIndex
  (CallFunction|SetIndex (- (Variables|Default|GetSelectedIndex) 1)))

(fn SetIndex
  (params (Index :type Integer))
  (Variables|Default|SetSelectedIndex (Math|Integer|SelectInt (Math|Integer|SelectInt (- (Variables|Default|GetOptionCount) 1) Index (< Index 0)) (Math|Integer|SelectInt -1 0 (<= (Variables|Default|GetOptionCount) 0)) (< Index (Variables|Default|GetOptionCount)))))