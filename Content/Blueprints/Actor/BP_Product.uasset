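; BP_Product is a product actor whose shape and color can be set at runtime through a static mesh component.
; SetShape and SetColor only write the Mesh and Material variables, with Color assigned directly as the material.
; RepNotify functions apply the changes to the component, keeping the appearance in sync across the network.
; The mesh notify also reapplies the material to slot 0 after swapping the mesh.
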(fn ConstructionScript)

(fn SetColor
  (params (Color :type Material%20Interface%20Object%20Reference))
  (Variables|Default|SetMaterial Color))

(fn SetShape
  (params (Mesh :type Static%20Mesh%20Object%20Reference))
  (Variables|Default|SetMesh Mesh))

(fn OnRepMesh
  (Components|StaticMesh|SetStaticMesh (Variables|Default|GetStaticMesh) (Variables|Default|GetMesh))
  (Rendering|Material|SetMaterial (Variables|Default|GetStaticMesh) 0 (Variables|Default|GetMaterial)))

(fn OnRepMaterial
  (bind _staticmesh (Variables|Default|GetStaticMesh)
    (:then
      (Rendering|Material|SetMaterial _staticmesh 0 (Variables|Default|GetMaterial)))
    (:else)))