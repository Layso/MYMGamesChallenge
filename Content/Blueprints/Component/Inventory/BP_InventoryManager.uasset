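; Inventory manager component that holds a single item at a time.
; AddItem fills the slot only when it is empty, and RemoveItem clears it only when given the held item.
; CurrentItem uses a RepNotify to fire the OnItemAdded and OnItemRemoved dispatchers, caching PreviousItem so the removal event can still pass the cleared item.
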(fn OnRepCurrentItem
  (bind _currentitem (Variables|Default|GetCurrentItem)
    (:then
      (bind _output_get (Variables|Default|SetPreviousItem _currentitem))
      (Default|CallOnItemAdded _output_get))
    (:else
      (Default|CallOnItemRemoved (Variables|Default|GetPreviousItem))
      (Variables|Default|SetPreviousItem 0))))

(fn HasItem
  (return (Utilities|IsValid (Variables|Default|GetCurrentItem))))

(fn GetItem
  (return (Variables|Default|GetCurrentItem)))

(fn AddItem
  (params (Item :type BP%20Inventory%20Item%20Object%20Reference))
  (Utilities|IsValid Item
    (:Is%20Valid
      (if (not (CallFunction|HasItem))
        (Variables|Default|SetCurrentItem Item)))))

(fn RemoveItem
  (params (Item :type BP%20Inventory%20Item%20Object%20Reference))
  (bind _currentitem (Variables|Default|GetCurrentItem)
    (:then
      (if (== _currentitem Item)
        (Variables|Default|SetCurrentItem 0)))
    (:else)))