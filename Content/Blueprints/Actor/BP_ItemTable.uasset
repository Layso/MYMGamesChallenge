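; Table actor that holds a single item, placed from the interacting player's inventory.
; On interaction it takes the item from the owner's BP_InventoryManager and snaps it to ItemSocket, raised by its bounds half-height.
; Placement blocks further interaction, binds to the item's added-to-inventory event and fires OnItemPlaced.
; OnItemTaken clears the slot and unblocks interaction, while GetItem exposes the current item.
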(event OnInteractionStarted(BP_Interactable)
  (params (Interactor :type BP%20Interactor%20Object%20Reference) (Component :type Primitive%20Component%20Object%20Reference))
  (CallFunction|TryPlaceItem Interactor))

(event EventBeginPlay
  (Networking|SwitchHasAuthority
    (:Authority
      (bind _bp_interactable (Variables|Default|GetBP_Interactable)
        (:then
          (Default|SetDefaultAimLabel _bp_interactable "Label_PlaceItem"))
        (:else)))))

(fn ConstructionScript)

(fn PlaceItem
  (params (Item :type Actor%20Object%20Reference))
  (if (CallFunction|IsEmpty)
    (bind _itemsocket (Variables|Default|GetItemSocket)
      (:then
        (bind _output_get (Variables|Default|SetCurrentItem Item))
        (Transformation|SetActorTransform _output_get (Math|Transform|MakeTransform (+ (.location (Transformation|GetWorldTransform _itemsocket)) (Math|Vector|MakeVector 0.0 0.0 (.z (.BoxExtent (Collision|GetActorBounds _output_get false false))))) (.rotation (Transformation|GetWorldTransform _itemsocket)) (.scale (Transformation|GetWorldTransform _itemsocket))))
        (Default|SetInteractionBlocked (Variables|Default|GetBP_Interactable) true)
        (Utilities|FlowControl|Sequence
          (:then_0
            (Utilities|IsValid (Actor|GetComponentbyClass (Variables|Default|GetCurrentItem) "/Game/Blueprints/Component/Inventory/BP_InventoryItem.BP_InventoryItem_C")
              (:Is%20Valid
                (EventDispatchers|BindEventtoOnAddedtoInventory (Actor|GetComponentbyClass (Variables|Default|GetCurrentItem) "/Game/Blueprints/Component/Inventory/BP_InventoryItem.BP_InventoryItem_C") (EventDispatchers|CreateEvent :!event OnItemTaken)))))
          (:then_1
            (Default|CallOnItemPlaced))))
      (:else))))

(fn IsEmpty
  (return (not (Utilities|IsValid (Variables|Default|GetCurrentItem)))))

(fn OnItemTaken
  (Variables|Default|SetCurrentItem 0)
  (Default|SetInteractionBlocked (Variables|Default|GetBP_Interactable) false))

(fn TryPlaceItem
  (params (Interactor :type BP%20Interactor%20Object%20Reference))
  (bind _returnvalue (Components|GetOwner Interactor))
  (Utilities|IsValid Interactor
    (:Is%20Valid
      (Utilities|IsValid _returnvalue
        (:Is%20Valid
          (bind _output_get (LocalVariables|SetInventory (Actor|GetComponentbyClass _returnvalue "/Game/Blueprints/Component/Inventory/BP_InventoryManager.BP_InventoryManager_C")))
          (Utilities|IsValid _output_get
            (:Is%20Valid
              (bind _output_get_2 (LocalVariables|SetItem (Default|GetItem _output_get)))
              (Utilities|IsValid _output_get_2
                (:Is%20Valid
                  (Default|RemoveItem (LocalVariables|GetInventory) (LocalVariables|GetItem))
                  (CallFunction|PlaceItem (Components|GetOwner (LocalVariables|GetItem))))))))))))

(fn GetItem
  (return (Variables|Default|GetCurrentItem)))