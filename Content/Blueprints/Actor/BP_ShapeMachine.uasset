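; BP_ShapeMachine is a machine actor that produces shape products chosen on a linked control panel.
; On authority, it builds its options from a ShapeList's map keys and binds the panel's selection and enter events.
; Selection changes show the shape's name, or an error, on the Monitor.
; Enter spawns a product at a socket point, sets its shape and places it on the OutputTable, only when that table is empty.
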(event EventBeginPlay
  (Networking|SwitchHasAuthority
    (:Authority
      (CallFunction|BindEvents)
      (CallFunction|GenerateShapeData)
      (bind _controlpanel (Variables|Default|GetControlPanel)
        (:then
          (Default|SetOptionCount _controlpanel (Utilities|Array|Length (Variables|Default|GetShapes))))
        (:else)))))

(fn ConstructionScript)

(fn BindEvents
  (Utilities|FlowControl|Sequence
    (:then_0
      (Variables|Default|GetControlPanel
        (:then
          (EventDispatchers|BindEventtoOnSelectionUpdated (Variables|Default|GetControlPanel) (EventDispatchers|CreateEvent :!event OnSelectionUpdated))
          (EventDispatchers|BindEventtoOnEnterButtonPressed (Variables|Default|GetControlPanel) (EventDispatchers|CreateEvent :!event OnEnterButtonPressed)))
        (:else)))))

(fn GenerateShapeData
  (bind _shapelist (Variables|Config|GetShapeList)
    (:then
      (bind _output_get (Variables|Default|SetNames (Variables|/Game/Blueprints/Data/DataAsset/Classes/DA_Class_ShapeList.DA_Class_ShapeList_C|GetShapes _shapelist)))
      (bind _keys (Utilities|Map|Keys _output_get))
      (Variables|Default|SetShapes _keys))
    (:else)))

(fn OnSelectionUpdated
  (params (Index :type Integer))
  (bind _shapes (Variables|Default|GetShapes))
  (bind _names (Variables|Default|GetNames))
  (bind _monitor (Variables|Default|GetMonitor))
  (bind _output (Utilities|Array|Get(acopy) _shapes Index))
  (bind (_value _returnvalue) (Utilities|Map|Find _names _output))
  (Variables|Default|GetControlPanel
    (:then
      (if (Utilities|Array|IsValidIndex (Variables|Default|GetShapes) Index)
        (if _returnvalue
          (Default|DisplayText _monitor _value)
          (else
            (Default|DisplayError _monitor :!label _label)))
        (else
          (goto _label))))
    (:else)))

(fn OnEnterButtonPressed
  (Variables|Default|GetControlPanel
    (:then
      (bind _outputtable (Variables|Default|GetOutputTable)
        (:then
          (if (and (Default|IsEmpty _outputtable) (Utilities|Array|IsValidIndex (Variables|Default|GetShapes) (Default|GetSelectedIndex (Variables|Default|GetControlPanel))))
            (bind _socket_spawnpoint (Variables|Default|GetSocket_SpawnPoint)
              (:then
                (bind _returnvalue (Game|SpawnActorfromClass (Variables|Config|GetProductActorClass) (Math|Transform|MakeTransform (.location (Transformation|GetWorldTransform _socket_spawnpoint)) (.rotation (Transformation|GetWorldTransform _socket_spawnpoint)) (Class|KismetMathLibrary|VectorOne)) "AlwaysSpawn" "MultiplyWithRoot" 0 0))
                (bind _output_get (LocalVariables|SetProduct _returnvalue))
                (Utilities|IsValid _output_get
                  (:Is%20Valid
                    (Default|SetShape (LocalVariables|GetProduct) (Utilities|Array|Get(acopy) (Variables|Default|GetShapes) (Default|GetSelectedIndex (Variables|Default|GetControlPanel))))
                    (Default|PlaceItem (Variables|Default|GetOutputTable) (LocalVariables|GetProduct)))))
              (:else))))
        (:else)))
    (:else)))