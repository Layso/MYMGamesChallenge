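; BP_GarbageBin is an interactable bin actor that destroys the item held by whoever uses it.
; On BeginPlay, the authority sets the interactable component's default aim label to the "Label_Destroy" key.
; When interaction starts, it finds the inventory manager on the interactor's owner, removes the item that manager returns, and destroys that item's owning actor.
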(event OnInteractionStarted(BP_Interactable)
  (params (Interactor :type BP%20Interactor%20Object%20Reference) (Component :type Primitive%20Component%20Object%20Reference))
  (CallFunction|TryDestroyItem Interactor))

(event EventBeginPlay
  (Networking|SwitchHasAuthority
    (:Authority
      (bind _bp_interactable (Variables|Default|GetBP_Interactable)
        (:then
          (Default|SetDefaultAimLabel _bp_interactable "Label_Destroy"))
        (:else)))))

(fn ConstructionScript)

(fn TryDestroyItem
  (params (Interactor :type BP%20Interactor%20Object%20Reference))
  (bind _returnvalue (Components|GetOwner Interactor))
  (Utilities|IsValid Interactor
    (:Is%20Valid
      (Utilities|IsValid _returnvalue
        (:Is%20Valid
          (bind _output_get (LocalVariables|SetInventory (Actor|GetComponentbyClass _returnvalue "/Game/Blueprints/Component/Inventory/BP_InventoryManager.BP_InventoryManager_C")))
          (Utilities|IsValid _output_get
            (:Is%20Valid
              (bind _output_get_2 (LocalVariables|SetItem (Default|GetItem (LocalVariables|GetInventory))))
              (Utilities|IsValid _output_get_2
                (:Is%20Valid
                  (Default|RemoveItem (LocalVariables|GetInventory) (LocalVariables|GetItem))
                  (Utilities|IsValid (Components|GetOwner (LocalVariables|GetItem))
                    (:Is%20Valid
                      (Actor|DestroyActor (Components|GetOwner (LocalVariables|GetItem))))))))))))))