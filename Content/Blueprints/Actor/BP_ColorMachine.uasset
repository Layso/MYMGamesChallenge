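; BP_ColorMachine is a machine actor that applies a player-selected color to a product.
; On BeginPlay, the authority loads colors and names from ColorList, sets the ControlPanel option count and binds its events.
; Selection changes show the color name, or an error, on the Monitor.
; Enter recolors the BP_Product on InputTable and places it on OutputTable, provided that table is empty and the selection is valid.
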(event EventBeginPlay
  (Networking|SwitchHasAuthority
    (:Authority
      (CallFunction|BindEvents)
      (CallFunction|GenerateColorData)
      (bind _controlpanel (Variables|Default|GetControlPanel)
        (:then
          (Default|SetOptionCount _controlpanel (Utilities|Array|Length (Variables|Default|GetColors))))
        (:else)))))

(fn ConstructionScript)

(fn BindEvents
  (Utilities|FlowControl|Sequence
    (:then_0
      (bind _controlpanel (Variables|Default|GetControlPanel)
        (:then
          (EventDispatchers|BindEventtoOnSelectionUpdated _controlpanel (EventDispatchers|CreateEvent :!event OnSelectionUpdated))
          (EventDispatchers|BindEventtoOnEnterButtonPressed (Variables|Default|GetControlPanel) (EventDispatchers|CreateEvent :!event OnEnterButtonPressed)))
        (:else)))))

(fn GenerateColorData
  (bind _colorlist (Variables|Config|GetColorList)
    (:then
      (bind _output_get (Variables|Default|SetNames (Variables|/Game/Blueprints/Data/DataAsset/Classes/DA_Class_ColorList.DA_Class_ColorList_C|GetColors _colorlist)))
      (bind _keys (Utilities|Map|Keys _output_get))
      (Variables|Default|SetColors _keys))
    (:else)))

(fn OnSelectionUpdated
  (params (Index :type Integer))
  (bind _names (Variables|Default|GetNames))
  (bind _colors (Variables|Default|GetColors))
  (bind _monitor (Variables|Default|GetMonitor))
  (bind _output (Utilities|Array|Get(acopy) _colors Index))
  (bind (_value _returnvalue) (Utilities|Map|Find _names _output))
  (Variables|Default|GetControlPanel
    (:then
      (if (Utilities|Array|IsValidIndex (Variables|Default|GetColors) Index)
        (if _returnvalue
          (Default|DisplayText _monitor _value)
          (else
            (Default|DisplayError _monitor :!label _label)))
        (else
          (goto _label))))
    (:else)))

(fn OnEnterButtonPressed
  (Variables|Default|GetControlPanel
    (:then
      (bind _outputtable (Variables|Default|GetOutputTable)
        (:then
          (if (and (Default|IsEmpty _outputtable) (Utilities|Array|IsValidIndex (Variables|Default|GetColors) (Default|GetSelectedIndex (Variables|Default|GetControlPanel))))
            (bind _inputtable (Variables|Default|GetInputTable)
              (:then
                (Utilities|IsValid (Default|GetItem _inputtable)
                  (:Is%20Valid
                    (bind _asbp_product (Utilities|Casting|CastToBP_Product (Default|GetItem _inputtable)))
                    (Default|SetColor _asbp_product (Utilities|Array|Get(acopy) (Variables|Default|GetColors) (Default|GetSelectedIndex (Variables|Default|GetControlPanel))))
                    (Default|PlaceItem (Variables|Default|GetOutputTable) _asbp_product))))
              (:else))))
        (:else)))
    (:else)))