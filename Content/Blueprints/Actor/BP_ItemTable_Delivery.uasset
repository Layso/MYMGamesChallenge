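; BP_ItemTable_Delivery is a delivery table that turns a placed product into a payment in the carpentry game.
; On the authority it binds to the item-placed event at BeginPlay.
; Product placement blocks the item's BP_Interactable and starts a timer standing in for a visual effect.
; The timer-end handler requests payment from BP_GameState_Carpentry, destroys the item and calls OnItemTaken to release the table.
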(event Custom|OnItemPlaced_Event)

(event EventBeginPlay
  (|CallParentFunction)
  (Networking|SwitchHasAuthority
    (:Authority
      (EventDispatchers|BindEventtoOnItemPlaced (EventDispatchers|CreateEvent :!event OnProductPlaced)))))

(fn ConstructionScript
  (|CallParentFunction))

(fn OnProductPlaced
  (bind _currentitem (Variables|Default|GetCurrentItem)
    (:then
      (Utilities|IsValid (Actor|GetComponentbyClass _currentitem "/Game/Blueprints/Component/BP_Interactable.BP_Interactable_C")
        (:Is%20Valid
          (Default|SetInteractionBlocked (Actor|GetComponentbyClass _currentitem "/Game/Blueprints/Component/BP_Interactable.BP_Interactable_C") true)
          (bind _returnvalue (Utilities|Time|SetTimerbyEvent (EventDispatchers|CreateEvent :!event OnVisualEffectTimerEnded) (Variables|Config|GetFakeVisualEffectTime)))
          (Variables|Default|SetFakeVisualEffectİmerHandle _returnvalue))))
    (:else)))

(fn OnVisualEffectTimerEnded
  (Utilities|FlowControl|Sequence
    (:then_0
      (bind _asbp_game_state_carpentry (Utilities|Casting|CastToBP_GameState_Carpentry (Game|GetGameState)))
      (Default|RequestPayment _asbp_game_state_carpentry (Variables|Default|GetCurrentItem)))
    (:then_1
      (bind _currentitem (Variables|Default|GetCurrentItem)
        (:then
          (Actor|DestroyActor _currentitem))
        (:else)))
    (:then_2
      (CallFunction|OnItemTaken))))