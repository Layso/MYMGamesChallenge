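; BP_InventoryItem, under the inventory component folder, tracks which inventory an item currently belongs to and announces changes in that membership.
; Notify functions set the CurrentInventory reference on addition and clear it on removal only if the given inventory is valid and matches.
; The RepNotify on that reference fires OnAddedToInventory when it is valid and OnRemovedFromInventory otherwise, so events follow the replicated state.
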(fn OnRepCurrentInventory
  (Variables|Default|GetCurrentInventory
    (:then
      (Default|CallOnAddedtoInventory))
    (:else
      (Default|CallOnRemovedfromInventory))))

(fn NotifyAddedtoInventory
  (params (Inventory :type BP%20Inventory%20Manager%20Object%20Reference))
  (Variables|Default|SetCurrentInventory Inventory))

(fn NotifyRemovedfromInventory
  (params (Inventory :type BP%20Inventory%20Manager%20Object%20Reference))
  (Utilities|IsValid Inventory
    (:Is%20Valid
      (if (== (Variables|Default|GetCurrentInventory) Inventory)
        (Variables|Default|SetCurrentInventory 0)))))