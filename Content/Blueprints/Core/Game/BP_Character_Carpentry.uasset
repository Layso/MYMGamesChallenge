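; Player character Blueprint for the Carpentry game, handling movement, look and interaction through Enhanced Input actions.
; Move input drives movement along the actor's right and forward vectors, while rotate input feeds controller yaw and pitch.
; Interact input starts an interaction on the BPInteractor component when it is valid.
; Eye viewpoint uses the CameraSocket location, falling back to actor location, with base aim rotation; local net ownership mirrors local control.
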(event Input|EnhancedActionEvents|EnhancedInputActionIA_Move
  (params (ActionValue :type Vector%202D%20Structure) (ElapsedSeconds :type Float%20%28double-precision%29) (TriggeredSeconds :type Float%20%28double-precision%29) (InputAction :type Input%20Action%20Object%20Reference :default "/Game/Input/Actions/IA_Move.IA_Move"))
  (bind (_x _y) (Math|Vector2D|BreakVector2D ActionValue))
  (Pawn|Input|AddMovementInput (Transformation|GetActorRightVector) _x false)
  (Pawn|Input|AddMovementInput (Transformation|GetActorForwardVector) _y false))

(event Input|EnhancedActionEvents|EnhancedInputActionIA_Rotate
  (params (ActionValue :type Vector%202D%20Structure) (ElapsedSeconds :type Float%20%28double-precision%29) (TriggeredSeconds :type Float%20%28double-precision%29) (InputAction :type Input%20Action%20Object%20Reference :default "/Game/Input/Actions/IA_Rotate.IA_Rotate"))
  (bind (_x _y) (Math|Vector2D|BreakVector2D ActionValue))
  (Pawn|Input|AddControllerYawInput _x)
  (Pawn|Input|AddControllerPitchInput _y))

(event Input|EnhancedActionEvents|EnhancedInputActionIA_Interact
  (params (ActionValue :type Boolean) (ElapsedSeconds :type Float%20%28double-precision%29) (TriggeredSeconds :type Float%20%28double-precision%29) (InputAction :type Input%20Action%20Object%20Reference :default "/Game/Input/Actions/IA_Interact.IA_Interact"))
  (bind _bp_interactor (Variables|Default|GetBP_Interactor)
    (:then
      (Default|StartInteraction _bp_interactor))
    (:else)))

(fn ConstructionScript)

(fn GetActorEyesViewPointBP
  (bind _returnvalue (Pawn|GetBaseAimRotation))
  (bind _camerasocket (Variables|Default|GetCameraSocket)
    (:then
      (return (Transformation|GetWorldLocation _camerasocket) _returnvalue))
    (:else
      (return (Transformation|GetActorLocation) _returnvalue))))

(fn HasLocalNetOwnerBP
  (return (Pawn|IsLocallyControlled)))