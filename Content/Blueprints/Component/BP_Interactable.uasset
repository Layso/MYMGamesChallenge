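; BP_Interactable is a component that marks its owning actor as interactable and receives interaction and aim notifications.
; CanInteract accepts any valid interactor unless the InteractionBlocked flag, set through SetInteractionBlocked, is on.
; The notify functions for interaction start and aim start, update and end only print debug messages.
; The interaction message names both owners, while aim messages take no interactor and name the component's owner twice.
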(event EventBeginPlay)

(event EventTick
  (params (DeltaSeconds :type Float%20%28single-precision%29)))

(fn CanInteract
  (params (Interactor :type BP%20Interactor%20Object%20Reference))
  (Utilities|IsValid Interactor
    (:Is%20Valid
      (return (not (Variables|Default|GetbInteractionBlocked))))
    (:Is%20Not%20Valid
      (return false))))

(fn SetInteractionBlocked
  (params (bBlocked :type Boolean))
  (Variables|Default|SetbInteractionBlocked bBlocked))

(fn NotifyInteractionStarted
  (params (Interactor :type BP%20Interactor%20Object%20Reference))
  (Development|PrintString (Utilities|String|Append (Utilities|GetDisplayName (Components|GetOwner Interactor)) " started interaction with " (Utilities|GetDisplayName (Components|GetOwner)))))

(fn NotifyAimStarted
  (Development|PrintString (Utilities|String|Append (Utilities|GetDisplayName (Components|GetOwner)) " started aim with " (Utilities|GetDisplayName (Components|GetOwner)))))

(fn NotifyAimUpdated
  (Development|PrintString (Utilities|String|Append (Utilities|GetDisplayName (Components|GetOwner)) " updated aim with " (Utilities|GetDisplayName (Components|GetOwner)))))

(fn NotifyAimEnded
  (Development|PrintString (Utilities|String|Append (Utilities|GetDisplayName (Components|GetOwner)) " ended aim with " (Utilities|GetDisplayName (Components|GetOwner)))))