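; Carpentry game state that holds the shared money and product order queue, replicating both to clients.
; On authority, a looping timer randomly adds orders with a random color and shape from the configured lists.
; RequestPayment consumes the oldest order, paying full price for matching shape and color, half for shape alone.
; RepNotifies broadcast money changes and diff orders by GUID to fire added, removed and updated events.
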(event EventBeginPlay
  (Networking|SwitchHasAuthority
    (:Authority
      (Variables|Default|SetMoney (Variables|Config|GetInitialMoney))
      (CallFunction|SetupOrderTimer))))

(fn ConstructionScript)

(fn GetActiveOrders
  (return (Variables|Default|GetActiveOrders_Replicated)))

(fn RequestPayment
  (params (Product :type Actor%20Object%20Reference))
  (if (Utilities|Array|IsNotEmpty (Variables|Default|GetActiveOrders_Replicated))
    (LocalVariables|SetOrder (Utilities|Array|Get(acopy) (Variables|Default|GetActiveOrders_Replicated)))
    (Utilities|Array|RemoveIndex (Variables|Default|GetActiveOrders_Replicated))
    (Variables|Default|SetActiveOrders_Replicated (Variables|Default|GetActiveOrders_Replicated))
    (bind _asbp_product (Utilities|Casting|CastToBP_Product Product))
    (if (== (Default|GetShape _asbp_product) (.Shape (Utilities|Struct|BreakSOrder (LocalVariables|GetOrder))))
      (if (== (.Color (Utilities|Struct|BreakSOrder (LocalVariables|GetOrder))) (Default|GetColor _asbp_product))
        (Variables|Default|SetMoney (+ (Variables|Default|GetMoney) (.Price (Utilities|Struct|BreakSOrder (LocalVariables|GetOrder)))))
        (else
          (Variables|Default|SetMoney (+ (Variables|Default|GetMoney) (/ (.Price (Utilities|Struct|BreakSOrder (LocalVariables|GetOrder))) 2))))))))

(fn SetupOrderTimer
  (bind _returnvalue (Utilities|Time|SetTimerbyEvent (EventDispatchers|CreateEvent :!event OnOrderTimerTriggered) (Variables|Config|GetOrderTimerInterval) true))
  (Variables|Default|SetOrderTimerHandle _returnvalue))

(fn OnOrderTimerTriggered
  (if (Math|Random|RandomBoolwithWeight (Variables|Config|GetOrderCreationPercentage))
    (bind _colorlist (Variables|Config|GetColorList)
      (:then
        (bind _keys (Utilities|Map|Keys (Variables|/Game/Blueprints/Data/DataAsset/Classes/DA_Class_ColorList.DA_Class_ColorList_C|GetColors _colorlist)))
        (LocalVariables|SetColor (.OutItem (Utilities|Array|Random _keys)))
        (bind _shapelist (Variables|Config|GetShapeList)
          (:then
            (bind _keys_2 (Utilities|Map|Keys (Variables|/Game/Blueprints/Data/DataAsset/Classes/DA_Class_ShapeList.DA_Class_ShapeList_C|GetShapes _shapelist)))
            (LocalVariables|SetShape (.OutItem (Utilities|Array|Random _keys_2)))
            (if (and (Utilities|IsValid (LocalVariables|GetColor)) (Utilities|IsValid (LocalVariables|GetShape)))
              (Utilities|Array|Add (Variables|Default|GetActiveOrders_Replicated) (Utilities|Struct|MakeSOrder (Guid|NewGuid) (LocalVariables|GetShape) (LocalVariables|GetColor) (Utilities|Time|GetTimeSeconds) (Variables|Config|GetDefaultProductPrice)))
              (Variables|Default|SetActiveOrders_Replicated (Variables|Default|GetActiveOrders_Replicated))))
          (:else)))
      (:else))))

(fn OnRepActiveOrdersReplicated
  (for _array_element (Variables|Default|GetActiveOrders_Replicated)
    (Utilities|Map|Add (LocalVariables|GetUpdatedList) (Utilities|Struct|BreakSOrder _array_element) _array_element))
  (Utilities|FlowControl|Sequence
    (:then_0
      (bind _keys (Utilities|Map|Keys (LocalVariables|GetUpdatedList)))
      (for _array_element_2 _keys
        (if (and (not (Utilities|Map|Contains (Variables|Default|GetActiveOrders) _array_element_2)) (.ReturnValue (Utilities|Map|Find (LocalVariables|GetUpdatedList) _array_element_2)))
          (Default|CallOnOrderAdded (.Value (Utilities|Map|Find (LocalVariables|GetUpdatedList) _array_element_2))))))
    (:then_1
      (bind _keys_2 (Utilities|Map|Keys (Variables|Default|GetActiveOrders)))
      (for _array_element_3 _keys_2
        (if (and (not (Utilities|Map|Contains (LocalVariables|GetUpdatedList) _array_element_3)) (.ReturnValue (Utilities|Map|Find (Variables|Default|GetActiveOrders) _array_element_3)))
          (Default|CallOnOrderRemoved (.Value (Utilities|Map|Find (Variables|Default|GetActiveOrders) _array_element_3))))))
    (:then_2
      (bind _output_get (Variables|Default|SetActiveOrders (LocalVariables|GetUpdatedList)))
      (Default|CallOnOrdersUpdated _output_get))))

(fn OnRepMoney
  (Default|CallOnMoneyUpdated (Variables|Default|GetMoney)))